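; Game mode for a Crossy Road-style game that tracks score and punishes an idle player with an eagle.
; AddScore starts the game on its first call, increments the score and timestamps the last move.
; Tick spawns BP_Eagle once, offset from the player's mesh, when a living player exceeds TimeBeforeDeath without scoring.
; SetHighScore copies a new best score into the GameInstance cached at BeginPlay.
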(event EventBeginPlay
  (bind _asgi_crossy_road (Utilities|Casting|CastToGI_CrossyRoad (Game|GetGameInstance)))
  (Variables|Default|SetGameInstanceREF _asgi_crossy_road))

(event EventTick
  (params (DeltaSeconds :type Float%20%28single-precision%29))
  (bind _returnvalue (Game|GetPlayerCharacter 0))
  (bind _mesh (Variables|/Script/Engine.Character|GetMesh _returnvalue))
  (bind _returnvalue_2 (Transformation|GetWorldTransform _mesh))
  (bind (_x _y _z) (Math|Vector|BreakVector (.location _returnvalue_2)))
  ;[1 1 1] Check if game started
  (if (Variables|Default|GetGameStarted)
    ;[1 1 1] Check if chicken is not dead
    (bind _asch_player (Utilities|Casting|CastToCH_Player (Game|GetPlayerCharacter 0)))
    (if (not (Variables|/Game/CrossyRoad/Blueprints/Character/CH_Player.CH_Player_C|GetisDead _asch_player))
      ;[1 1 1] If Haven't Moved Before Timer, Spawn Eagle
      (if (>= (- (Utilities|Time|GetTimeSeconds) (Variables|Default|GetLastMovedUp)) (Variables|Default|GetTimeBeforeDeath))
        (Utilities|FlowControl|DoOnce false
          (:Completed
            (Development|PrintString "SPAWN EAGLE!!!")
            (Game|SpawnActorfromClass "/Game/CrossyRoad/Blueprints/Obstacles/BP_Eagle.BP_Eagle_C" (Math|Transform|MakeTransform (Math|Vector|MakeVector (+ _x 1e+03) _y (+ _z 1e+03)) "0.0,90.000000,0.0" (.scale _returnvalue_2)) "Undefined" 0 _returnvalue 0)))))))

(fn ConstructionScript)

(fn SetHighScore
  (if (> (Variables|Default|GetScore) (Variables|/Game/CrossyRoad/Blueprints/Core/GI_CrossyRoad.GI_CrossyRoad_C|GetHighScore (Variables|Default|GetGameInstanceREF)))
    (Variables|/Game/CrossyRoad/Blueprints/Core/GI_CrossyRoad.GI_CrossyRoad_C|SetHighScore (Variables|Default|GetGameInstanceREF) (Variables|Default|GetScore))))

(fn AddScore
  (if (Variables|Default|GetGameStarted)
    (Math|Integer|IncrementInt (Variables|Default|GetScore)
      (:%20%20
        (Variables|Default|SetLastMovedUp (Utilities|Time|GetTimeSeconds))))
    (else
      (Variables|Default|SetLastMovedUp (Utilities|Time|GetTimeSeconds))
      (Variables|Default|SetGameStarted true)
      (Math|Integer|IncrementInt (Variables|Default|GetScore)))))