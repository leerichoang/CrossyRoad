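; BP_Truck is a moving road obstacle for the Crossy Road game that kills the player's chicken on contact.
; On spawn it gives the car mesh a random paint material and sets a lifespan, then Tick sweeps the root along world Y at SpeedValue.
; When the car overlaps CH_Player, it calls ChickenRoadKill and opens L_CrossRoad after a short delay.
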(event OnComponentBeginOverlap(Car)
  (params (OverlappedComponent :type Primitive%20Component%20Object%20Reference) (OtherActor :type Actor%20Object%20Reference) (OtherComp :type Primitive%20Component%20Object%20Reference) (OtherBodyIndex :type Integer) (bFromSweep :type Boolean) (SweepResult :type Hit%20Result%20Structure%20%28by%20ref%29))
  (bind _asch_player (Utilities|Casting|CastToCH_Player OtherActor))
  (Default|ChickenRoadKill _asch_player)
  (Utilities|FlowControl|Delay 2.0)
  (Game|OpenLevel(byName) "L_CrossRoad"))

(event EventBeginPlay
  (Rendering|Material|SetMaterial (Variables|Default|GetCar) 0 (Utilities|Select :Index (Math|Random|RandomIntegerinRange 0 4) :Option%200 "/Game/CrossyRoad/Materials/BluePaint.BluePaint" :Option%201 "/Game/CrossyRoad/Materials/M_RED.M_RED" :Option%202 "/Game/CrossyRoad/Materials/M_ORANGE.M_ORANGE" :Option%203 "/Game/CrossyRoad/Materials/RedPaint.RedPaint" :Option%204 "/Game/CrossyRoad/Materials/M_WhiteFeather.M_WhiteFeather"))
  (Actor|SetLifeSpan (Variables|Default|GetLifeSpan)))

(event Collision|EventActorBeginOverlap
  (params (OtherActor :type Actor%20Object%20Reference)))

(event EventTick
  (params (DeltaSeconds :type Float%20%28single-precision%29))
  (Transformation|AddWorldOffset (Variables|Default|GetDefaultSceneRoot) (Math|Vector|MakeVector 0.0 (* DeltaSeconds (Variables|Default|GetSpeedValue)) 0.0) true false))

(fn ConstructionScript)