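; BP_PlatformSpawner builds the starting strip of platforms for the Crossy Road level.
; On BeginPlay it destroys existing BP_Platform actors, then spawns a short chain beginning with a regular platform at a fixed location.
; Each following platform is randomly regular, street or water, placed at the previous one's SpawnPoint.
; It tracks the newest platform and hands each spawned platform a reference back to itself.
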(event EventBeginPlay
  (CallFunction|SpawnInitialPlatform))

(event Collision|EventActorBeginOverlap
  (params (OtherActor :type Actor%20Object%20Reference)))

(event EventTick
  (params (DeltaSeconds :type Float%20%28single-precision%29)))

(fn ConstructionScript)

(fn SpawnInitialPlatform
  (Utilities|FlowControl|Sequence
    (:then_0
      (bind _outactors (Actor|GetAllActorsOfClass "/Game/CrossyRoad/Blueprints/Obstacles/BP_Platform.BP_Platform_C"))
      (for _array_element _outactors
        (Actor|DestroyActor _array_element)))
    (:then_1
      (for _index (range 0 5)
        (Utilities|IsValid (Variables|Default|GetNewestPlatform)
          (:Is%20Valid
            (CallFunction|SpawnPlatformatSpawnPoint))
          (:Is%20Not%20Valid
            (CallFunction|SpawnRegularPlatform)))))))

(fn SpawnPlatformatSpawnPoint
  (bind _asbp_platform (Utilities|Casting|CastToBP_Platform (Variables|Default|GetNewestPlatform)))
  (CallFunction|SpawnPlatform (Transformation|GetWorldLocation (Variables|/Game/CrossyRoad/Blueprints/Obstacles/BP_Platform.BP_Platform_C|GetSpawnPoint _asbp_platform))))

(fn SpawnPlatform
  (params (Spawn%20Location :type Vector))
  (bind _returnvalue (Game|SpawnActorfromClass (Utilities|Select :Index (Math|Random|RandomIntegerinRange 0 2) :Option%200 "/Game/CrossyRoad/Blueprints/Obstacles/BP_Platform.BP_Platform_C" :Option%201 "/Game/CrossyRoad/Blueprints/Obstacles/BP_Platform_Street.BP_Platform_Street_C" :Option%202 "/Game/CrossyRoad/Blueprints/Obstacles/BP_Platform_Water.BP_Platform_Water_C") (Math|Transform|MakeTransform Spawn%20Location "0, 0, 0" "1,1,1") "Undefined" 0 0))
  (bind _output_get (Variables|Default|SetNewestPlatform _returnvalue))
  (bind _asbp_platform (Utilities|Casting|CastToBP_Platform _output_get))
  (Variables|/Game/CrossyRoad/Blueprints/Obstacles/BP_Platform.BP_Platform_C|SetPlatformSpawner _asbp_platform self))

(fn SpawnRegularPlatform
  (bind _returnvalue (Game|SpawnActorfromClass "/Game/CrossyRoad/Blueprints/Obstacles/BP_Platform.BP_Platform_C" (Math|Transform|MakeTransform "-200.000000, 0, 0" "0, 0, 0" "1,1,1") "Undefined" 0 0))
  (bind _output_get (Variables|Default|SetNewestPlatform _returnvalue))
  (bind _asbp_platform (Utilities|Casting|CastToBP_Platform _output_get))
  (Variables|/Game/CrossyRoad/Blueprints/Obstacles/BP_Platform.BP_Platform_C|SetPlatformSpawner _asbp_platform self))