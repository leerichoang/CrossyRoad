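; Test obstacle platform for the Crossy Road game that populates itself with node actors at runtime.
; On BeginPlay it calls the parent, then GenerateNodes0 spawns a BP_Base_Node at the world transform of each of its fourteen Node components.
; The spawns are unrolled calls with no loop, and the spawned actors are not stored.
; Tick and overlap events are disabled, and the construction script only calls the parent.
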(event EventBeginPlay
  (|CallParentFunction)
  (CallFunction|GenerateNodes0))

(event Collision|EventActorBeginOverlap
  (params (OtherActor :type Actor%20Object%20Reference))
  (|CallParentFunction OtherActor) ; This node is disabled and will not be called.\nDrag off pins to build functionality.
)

(event EventTick
  (params (DeltaSeconds :type Float%20%28single-precision%29))
  (|CallParentFunction DeltaSeconds) ; This node is disabled and will not be called.\nDrag off pins to build functionality.
)

(fn ConstructionScript
  (|CallParentFunction))

(fn GenerateNodes0
  (Game|SpawnActorfromClass "/Game/CrossyRoad/Blueprints/BP_Base_Node.BP_Base_Node_C" (Transformation|GetWorldTransform (Variables|Default|GetNode%201)) "Undefined" 0 0)
  (Game|SpawnActorfromClass "/Game/CrossyRoad/Blueprints/BP_Base_Node.BP_Base_Node_C" (Transformation|GetWorldTransform (Variables|Default|GetNode%202)) "Undefined" 0 0)
  (Game|SpawnActorfromClass "/Game/CrossyRoad/Blueprints/BP_Base_Node.BP_Base_Node_C" (Transformation|GetWorldTransform (Variables|Default|GetNode%203)) "Undefined" 0 0)
  (Game|SpawnActorfromClass "/Game/CrossyRoad/Blueprints/BP_Base_Node.BP_Base_Node_C" (Transformation|GetWorldTransform (Variables|Default|GetNode%204)) "Undefined" 0 0)
  (Game|SpawnActorfromClass "/Game/CrossyRoad/Blueprints/BP_Base_Node.BP_Base_Node_C" (Transformation|GetWorldTransform (Variables|Default|GetNode%205)) "Undefined" 0 0)
  (Game|SpawnActorfromClass "/Game/CrossyRoad/Blueprints/BP_Base_Node.BP_Base_Node_C" (Transformation|GetWorldTransform (Variables|Default|GetNode%206)) "Undefined" 0 0)
  (Game|SpawnActorfromClass "/Game/CrossyRoad/Blueprints/BP_Base_Node.BP_Base_Node_C" (Transformation|GetWorldTransform (Variables|Default|GetNode%207)) "Undefined" 0 0)
  (Game|SpawnActorfromClass "/Game/CrossyRoad/Blueprints/BP_Base_Node.BP_Base_Node_C" (Transformation|GetWorldTransform (Variables|Default|GetNode%208)) "Undefined" 0 0)
  (Game|SpawnActorfromClass "/Game/CrossyRoad/Blueprints/BP_Base_Node.BP_Base_Node_C" (Transformation|GetWorldTransform (Variables|Default|GetNode%209)) "Undefined" 0 0)
  (Game|SpawnActorfromClass "/Game/CrossyRoad/Blueprints/BP_Base_Node.BP_Base_Node_C" (Transformation|GetWorldTransform (Variables|Default|GetNode%2010)) "Undefined" 0 0)
  (Game|SpawnActorfromClass "/Game/CrossyRoad/Blueprints/BP_Base_Node.BP_Base_Node_C" (Transformation|GetWorldTransform (Variables|Default|GetNode%2011)) "Undefined" 0 0)
  (Game|SpawnActorfromClass "/Game/CrossyRoad/Blueprints/BP_Base_Node.BP_Base_Node_C" (Transformation|GetWorldTransform (Variables|Default|GetNode%2012)) "Undefined" 0 0)
  (Game|SpawnActorfromClass "/Game/CrossyRoad/Blueprints/BP_Base_Node.BP_Base_Node_C" (Transformation|GetWorldTransform (Variables|Default|GetNode%2013)) "Undefined" 0 0)
  (Game|SpawnActorfromClass "/Game/CrossyRoad/Blueprints/BP_Base_Node.BP_Base_Node_C" (Transformation|GetWorldTransform (Variables|Default|GetNode%2014)) "Undefined" 0 0))