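; BP_Eagle is an eagle obstacle in a Crossy Road-style game that hunts and kills the player's chicken.
; Each Tick it steps by Speed toward the Player reference on each axis independently, comparing skeletal mesh and player positions, without delta-time scaling.
; When its Box overlaps CH_Player, it calls ChickenDeath and sets PlayerFound, switching Tick to a fixed upward retreat along negative X.
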(event OnComponentBeginOverlap(Box)
  (params (OverlappedComponent :type Primitive%20Component%20Object%20Reference) (OtherActor :type Actor%20Object%20Reference) (OtherComp :type Primitive%20Component%20Object%20Reference) (OtherBodyIndex :type Integer) (bFromSweep :type Boolean) (SweepResult :type Hit%20Result%20Structure%20%28by%20ref%29))
  (bind _asch_player (Utilities|Casting|CastToCH_Player OtherActor))
  (Variables|Default|SetPlayerFound true)
  (Default|ChickenDeath _asch_player))

(event EventBeginPlay)

(event Collision|EventActorBeginOverlap
  (params (OtherActor :type Actor%20Object%20Reference)))

(event EventTick
  (params (DeltaSeconds :type Float%20%28single-precision%29))
  (bind _skeletalmesh (Variables|Default|GetSkeletalMesh))
  (bind _player (Variables|Default|GetPlayer))
  (bind _speed (Variables|Default|GetSpeed))
  (bind _speed_2 (Variables|Default|GetSpeed))
  (bind _speed_3 (Variables|Default|GetSpeed))
  (bind _returnvalue (Transformation|GetWorldLocation _skeletalmesh))
  (bind _returnvalue_2 (Transformation|GetActorLocation _player))
  (if (not (Variables|Default|GetPlayerFound))
    ;[1 1 1] Attack Player
    (if (> (- (.x _returnvalue) (.x _returnvalue_2)) 0.0)
      (Variables|Default|SetXValue (* _speed_2 -1.0))
      (else
        (Variables|Default|SetXValue _speed_2)))
    (if (> (- (.y _returnvalue) (.y _returnvalue_2)) 0.0)
      (Variables|Default|SetYValue (* _speed_3 -1.0))
      (else
        (Variables|Default|SetYValue _speed_3)))
    (if (> (- (.z _returnvalue) (.z _returnvalue_2)) 0.0)
      (Variables|Default|SetZValue (* _speed -1.0))
      (else
        (Variables|Default|SetZValue _speed)))
    (Transformation|AddActorWorldOffset (Math|Vector|MakeVector (Variables|Default|GetXValue) (Variables|Default|GetYValue) (Variables|Default|GetZValue)))
    (else
      (Transformation|AddActorWorldOffset (Math|Vector|MakeVector -1e+01 0.0 1e+01)))))

(fn ConstructionScript)