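; Water lane platform in a Crossy Road-style game that sends floating logs across it from one side.
; On BeginPlay it randomly picks left or right, rolls a spawn interval and log speed, and starts a looping timer.
; Each timer tick spawns a BP_Log at that side's spawn point, negating its float speed for the right side.
; When the player overlaps the water collision, it only spawns an ice-shatter particle effect below them.
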(event OnComponentBeginOverlap(WaterCollision)
  (params (OverlappedComponent :type Primitive%20Component%20Object%20Reference) (OtherActor :type Actor%20Object%20Reference) (OtherComp :type Primitive%20Component%20Object%20Reference) (OtherBodyIndex :type Integer) (bFromSweep :type Boolean) (SweepResult :type Hit%20Result%20Structure%20%28by%20ref%29))
  (bind _asch_player (Utilities|Casting|CastToCH_Player OtherActor))
  (Effects|SpawnEmitteratLocation "/Game/InfinityBladeEffects/Effects/FX_Skill_Aura/P_Aura_Ice_Shatter_01.P_Aura_Ice_Shatter_01" (+ (.location (Transformation|GetActorTransform _asch_player)) "0, 0,-150.000000") (.rotation (Transformation|GetActorTransform _asch_player)) "0.500000,0.500000,1.000000"))

(event EventBeginPlay
  (bind _returnvalue (Math|Random|RandomFloatinRange 3.0 4.0))
  (|CallParentFunction)
  (bind _output_get (Variables|Default|SetbLeftSpawning (Math|Random|RandomBool)))
  (if _output_get
    ;[1 1 1] Left Log
    (bind _output_get_2 (Variables|Default|SetLeftLogSpawnRate _returnvalue))
    (Variables|Default|SetLeftLogSpeed (Math|Random|RandomFloatinRange 3e+02 7e+02))
    (Utilities|Time|SetTimerbyFunctionName 0 "CreateLeftLogs" _output_get_2 true)
    (else
      ;[1 1 1] Spawn Right
      (bind _output_get_3 (Variables|Default|SetRightLogSpawnRate _returnvalue))
      (Variables|Default|SetRightLogSpeed (Math|Random|RandomFloatinRange 3e+02 7e+02))
      (Utilities|Time|SetTimerbyFunctionName 0 "CreateRightLogs" _output_get_3 true))))

(event Collision|EventActorBeginOverlap
  (params (OtherActor :type Actor%20Object%20Reference))
  (|CallParentFunction OtherActor) ; This node is disabled and will not be called.\nDrag off pins to build functionality.
)

(event EventTick
  (params (DeltaSeconds :type Float%20%28single-precision%29))
  (|CallParentFunction DeltaSeconds) ; This node is disabled and will not be called.\nDrag off pins to build functionality.
)

(fn ConstructionScript
  (|CallParentFunction))

(fn CreateLeftLogs
  (bind _returnvalue (Game|SpawnActorfromClass "/Game/CrossyRoad/Blueprints/Obstacles/BP_Log.BP_Log_C" (Transformation|GetWorldTransform (Variables|Default|GetLogSpawnPoint)) "Undefined" 0 0))
  (Variables|/Game/CrossyRoad/Blueprints/Obstacles/BP_Log.BP_Log_C|SetFloatSpeed _returnvalue (Variables|Default|GetLeftLogSpeed)))

(fn CreateRightLogs
  (bind _returnvalue (Game|SpawnActorfromClass "/Game/CrossyRoad/Blueprints/Obstacles/BP_Log.BP_Log_C" (Transformation|GetWorldTransform (Variables|Default|GetLogSpawnPoint_02)) "Undefined" 0 0))
  (Variables|/Game/CrossyRoad/Blueprints/Obstacles/BP_Log.BP_Log_C|SetFloatSpeed _returnvalue (* (Variables|Default|GetRightLogSpeed) -1.0)))