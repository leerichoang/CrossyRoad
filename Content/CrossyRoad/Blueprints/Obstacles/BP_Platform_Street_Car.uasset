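; Street lane platform for a Crossy Road-style game that spawns a stream of BP_Car traffic from one randomly chosen side.
; BeginPlay rolls a spawn interval once for a looping Create Car timer, and derives car speed from that range, so sparser ranges move faster.
; Right-side spawns negate the speed, and the timer pauses on destruction.
; A player overlapping either side wall makes GM_CrossyRoad spawn the eagle.
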(event OnComponentBeginOverlap(LeftWall)
  (params (OverlappedComponent :type Primitive%20Component%20Object%20Reference) (OtherActor :type Actor%20Object%20Reference) (OtherComp :type Primitive%20Component%20Object%20Reference) (OtherBodyIndex :type Integer) (bFromSweep :type Boolean) (SweepResult :type Hit%20Result%20Structure%20%28by%20ref%29))
  (Utilities|Casting|CastToCH_Player (stale OnComponentBeginOverlap(RightWall) OtherActor))
  (bind _asgm_crossy_road (Utilities|Casting|CastToGM_CrossyRoad (Game|GetGameMode)))
  (Default|SpawnEagle _asgm_crossy_road))

(event OnComponentBeginOverlap(RightWall)
  (params (OverlappedComponent :type Primitive%20Component%20Object%20Reference) (OtherActor :type Actor%20Object%20Reference) (OtherComp :type Primitive%20Component%20Object%20Reference) (OtherBodyIndex :type Integer) (bFromSweep :type Boolean) (SweepResult :type Hit%20Result%20Structure%20%28by%20ref%29))
  (Utilities|Casting|CastToCH_Player OtherActor)
  (bind _asgm_crossy_road (Utilities|Casting|CastToGM_CrossyRoad (Game|GetGameMode)))
  (Default|SpawnEagle _asgm_crossy_road))

(event EventBeginPlay
  (|CallParentFunction)
  (Variables|Default|SetLeftSide (Math|Random|RandomBool))
  (bind _output_get (Variables|Default|SetMinSpawnRate (Math|Random|RandomIntegerinRange 2 5)))
  (bind _output_get_2 (Variables|Default|SetMaxSpawnRate (+ _output_get 4)))
  (Variables|Default|SetSpeed (Math|Conversions|ToFloat(Integer) (* _output_get_2 100)))
  (bind _output_get_3 (Variables|Default|SetRandomTimer (Math|Conversions|ToFloat(Integer) (Math|Random|RandomIntegerinRange (Variables|Default|GetMinSpawnRate) (Variables|Default|GetMaxSpawnRate)))))
  (Utilities|Time|SetTimerbyFunctionName 0 "Create Car" _output_get_3 true))

(event Collision|EventActorBeginOverlap
  (params (OtherActor :type Actor%20Object%20Reference))
  (|CallParentFunction OtherActor) ; This node is disabled and will not be called.\nDrag off pins to build functionality.
)

(event EventTick
  (params (DeltaSeconds :type Float%20%28single-precision%29))
  (|CallParentFunction DeltaSeconds) ; This node is disabled and will not be called.\nDrag off pins to build functionality.
)

(event EventDestroyed
  (Class|KismetSystemLibrary|PauseTimer 0 "Create Car"))

(fn ConstructionScript
  (|CallParentFunction))

(fn CreateCar
  (bind _speed (Variables|Default|GetSpeed))
  (if (Variables|Default|GetLeftSide)
    (Game|SpawnActorfromClass "/Game/CrossyRoad/Blueprints/Obstacles/BP_Car.BP_Car_C" (Transformation|GetWorldTransform (Variables|Default|GetCarSpawn)) "Undefined" 0 _speed 0)
    (else
      (bind _returnvalue (Game|SpawnActorfromClass "/Game/CrossyRoad/Blueprints/Obstacles/BP_Car.BP_Car_C" (Transformation|GetWorldTransform (Variables|Default|GetCarSpawn_02)) "Undefined" 0 _speed 0))
      (Variables|/Game/CrossyRoad/Blueprints/Obstacles/BP_Car.BP_Car_C|SetSpeedValue _returnvalue (* (Variables|/Game/CrossyRoad/Blueprints/Obstacles/BP_Car.BP_Car_C|GetSpeedValue _returnvalue) -1.0)))))