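; BP_Platform_Street_Truck is a street platform obstacle in a Crossy Road-style game that keeps spawning trucks.
; On BeginPlay it randomly picks a side, a spawn-rate range, a speed derived from that range, and a timer interval.
; A looping timer, fixed at that interval, calls Create Truck, which spawns BP_Truck at the chosen spawn point, negating its speed for one direction.
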(event EventBeginPlay
  (|CallParentFunction)
  (Variables|Default|SetLeftSide (Math|Random|RandomBool))
  (bind _output_get (Variables|Default|SetMinSpawnRate (Math|Random|RandomIntegerinRange 1 5)))
  (bind _output_get_2 (Variables|Default|SetMaxSpawnRate (+ _output_get 2)))
  (Variables|Default|SetSpeed (Math|Conversions|ToFloat(Integer) (* _output_get_2 125)))
  (bind _output_get_3 (Variables|Default|SetRandomTimer (Math|Conversions|ToFloat(Integer) (Math|Random|RandomIntegerinRange (Variables|Default|GetMinSpawnRate) (Variables|Default|GetMaxSpawnRate)))))
  (Utilities|Time|SetTimerbyFunctionName 0 "Create Truck" _output_get_3 true))

(event Collision|EventActorBeginOverlap
  (params (OtherActor :type Actor%20Object%20Reference))
  (|CallParentFunction OtherActor) ; This node is disabled and will not be called.\nDrag off pins to build functionality.
)

(event EventTick
  (params (DeltaSeconds :type Float%20%28single-precision%29))
  (|CallParentFunction DeltaSeconds) ; This node is disabled and will not be called.\nDrag off pins to build functionality.
)

(fn ConstructionScript
  (|CallParentFunction))

(fn CreateTruck
  (bind _speed (Variables|Default|GetSpeed))
  (if (Variables|Default|GetLeftSide)
    (Game|SpawnActorfromClass "/Game/CrossyRoad/Blueprints/Obstacles/BP_Truck.BP_Truck_C" (Transformation|GetWorldTransform (Variables|Default|GetTruckSpawnR)) "Undefined" 0 _speed 0)
    (else
      (bind _returnvalue (Game|SpawnActorfromClass "/Game/CrossyRoad/Blueprints/Obstacles/BP_Truck.BP_Truck_C" (Transformation|GetWorldTransform (Variables|Default|GetTruckSpawnL)) "Undefined" 0 _speed 0))
      (Variables|/Game/CrossyRoad/Blueprints/Obstacles/BP_Truck.BP_Truck_C|SetSpeedValue _returnvalue (* (Variables|/Game/CrossyRoad/Blueprints/Obstacles/BP_Truck.BP_Truck_C|GetSpeedValue _returnvalue) -1.0)))))