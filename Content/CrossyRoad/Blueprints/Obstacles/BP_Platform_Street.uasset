(event EventBeginPlay
  (|CallParentFunction)
  (Variables|Default|SetLeftSide (Math|Random|RandomBool))
  (bind _output_get (Variables|Default|SetRandomTimer (Math|Conversions|ToFloat(Integer) (Math|Random|RandomIntegerinRange 1 5))))
  (Utilities|Time|SetTimerbyFunctionName 0 "Create Car" _output_get true))

(event Collision|EventActorBeginOverlap
  (params (OtherActor :type Actor%20Object%20Reference))
  (|CallParentFunction OtherActor) ; This node is disabled and will not be called.\nDrag off pins to build functionality.
)

(event EventTick
  (params (DeltaSeconds :type Float%20%28single-precision%29))
  (|CallParentFunction DeltaSeconds) ; This node is disabled and will not be called.\nDrag off pins to build functionality.
)

(fn ConstructionScript
  (|CallParentFunction))

(fn CreateCar
  (if (Variables|Default|GetLeftSide)
    (Game|SpawnActorfromClass "/Game/CrossyRoad/Blueprints/Obstacles/BP_Car.BP_Car_C" (Transformation|GetWorldTransform (Variables|Default|GetCarSpawn)) "Undefined" 0 0)
    (else
      (bind _returnvalue (Game|SpawnActorfromClass "/Game/CrossyRoad/Blueprints/Obstacles/BP_Car.BP_Car_C" (Transformation|GetWorldTransform (Variables|Default|GetCarSpawn_02)) "Undefined" 0 0))
      (Variables|/Game/CrossyRoad/Blueprints/Obstacles/BP_Car.BP_Car_C|SetSpeedValue _returnvalue (* (Variables|/Game/CrossyRoad/Blueprints/Obstacles/BP_Car.BP_Car_C|GetSpeedValue _returnvalue) -1.0)))))