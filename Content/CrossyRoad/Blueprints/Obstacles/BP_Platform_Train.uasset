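; Train-track platform obstacle for a Crossy Road-style game that periodically sends a train across, preceded by flashing warning lights.
; On BeginPlay it randomly picks a side and a looping spawn interval, both then fixed for that platform.
; Each cycle starts a timer that alternates two point-light groups, then spawns BP_Train after a delay, negating its speed for left-side spawns.
; Despawn overlaps destroy the train, hide all lights and clear the flashing timer.
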(event OnComponentBeginOverlap(DespawnPoint1)
  (params (OverlappedComponent :type Primitive%20Component%20Object%20Reference) (OtherActor :type Actor%20Object%20Reference) (OtherComp :type Primitive%20Component%20Object%20Reference) (OtherBodyIndex :type Integer) (bFromSweep :type Boolean) (SweepResult :type Hit%20Result%20Structure%20%28by%20ref%29))
  (bind _asbp_train (Utilities|Casting|CastToBP_Train OtherActor))
  (Actor|DestroyActor _asbp_train)
  (CallFunction|TrainLightOff))

(event OnComponentBeginOverlap(DespawnPoint)
  (params (OverlappedComponent :type Primitive%20Component%20Object%20Reference) (OtherActor :type Actor%20Object%20Reference) (OtherComp :type Primitive%20Component%20Object%20Reference) (OtherBodyIndex :type Integer) (bFromSweep :type Boolean) (SweepResult :type Hit%20Result%20Structure%20%28by%20ref%29))
  (bind _asbp_train (Utilities|Casting|CastToBP_Train OtherActor))
  (Actor|DestroyActor _asbp_train)
  (CallFunction|TrainLightOff))

(event Custom|Create%20Train
  (bind _returnvalue (Utilities|Time|SetTimerbyFunctionName 0 "TrainLightOn" 0.5 true))
  (Variables|Default|SetTrain%20Light%20Handle _returnvalue)
  (if (Variables|Default|GetLeftSide)
    (Utilities|FlowControl|Delay 2.0)
    (bind _returnvalue_2 (Game|SpawnActorfromClass "/Game/CrossyRoad/Blueprints/Obstacles/BP_Train.BP_Train_C" (Transformation|GetWorldTransform (Variables|Default|GetTrainSpawn)) "Undefined" 0 9e+03 0 0))
    (Variables|/Game/CrossyRoad/Blueprints/Obstacles/BP_Train.BP_Train_C|SetSpeedValue _returnvalue_2 (* (Variables|/Game/CrossyRoad/Blueprints/Obstacles/BP_Train.BP_Train_C|GetSpeedValue _returnvalue_2) -1.0))
    (else
      (Utilities|FlowControl|Delay 2.0)
      (Game|SpawnActorfromClass "/Game/CrossyRoad/Blueprints/Obstacles/BP_Train.BP_Train_C" (Transformation|GetWorldTransform (Variables|Default|GetTrainSpawn1)) "Undefined" 0 9e+03 0 0))))

(event EventBeginPlay
  (|CallParentFunction)
  (Variables|Default|SetLeftSide (Math|Random|RandomBool))
  ;[1 1 1] Spawn Train
  (bind _output_get (Variables|Default|SetRandomTimer (Math|Conversions|ToFloat(Integer) (Math|Random|RandomIntegerinRange 6 10))))
  (Utilities|Time|SetTimerbyEvent (delegate Custom|Create%20Train) _output_get true))

(event Collision|EventActorBeginOverlap
  (params (OtherActor :type Actor%20Object%20Reference))
  (|CallParentFunction OtherActor) ; This node is disabled and will not be called.\nDrag off pins to build functionality.
)

(fn ConstructionScript
  (|CallParentFunction))

(fn TrainLighton
  (if (Variables|Default|GetbLeftLight)
    (Rendering|SetVisibility (Variables|Default|GetPointLight5) false false)
    (Rendering|SetVisibility (Variables|Default|GetPointLight) true false)
    (Variables|Default|SetbLeftLight false)
    (else
      (Rendering|SetVisibility (Variables|Default|GetPointLight5) true false)
      (Rendering|SetVisibility (Variables|Default|GetPointLight) false false)
      (Variables|Default|SetbLeftLight true))))

(fn TrainLightOff
  (Rendering|SetVisibility (Variables|Default|GetPointLight5) false false)
  (Utilities|Time|ClearandInvalidateTimerbyHandle (Variables|Default|GetTrain%20Light%20Handle)))