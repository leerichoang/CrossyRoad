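; BP_Platform_Lilypads is a Crossy Road platform that scatters lily pads across its nodes.
; On BeginPlay it draws a random number of picks from available nodes, using AddUnique so repeated picks collapse into fewer pads.
; It spawns BP_Lilypads at each chosen node, lowered by a Z offset, and marks that node occupied.
; Spawned pads are tracked in Obstacles and destroyed along with the platform.
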(event EventBeginPlay
  (|CallParentFunction)
  (CallFunction|SpawnLilyPads))

(event Collision|EventActorBeginOverlap
  (params (OtherActor :type Actor%20Object%20Reference)))

(event EventTick
  (params (DeltaSeconds :type Float%20%28single-precision%29))
  (|CallParentFunction DeltaSeconds) ; This node is disabled and will not be called.\nDrag off pins to build functionality.
)

(event EventDestroyed
  (CallFunction|DestroyObstacles))

(fn ConstructionScript
  (|CallParentFunction))

(fn SpawnLilyPads
  ;[1 1 1] Generate at most 7 block actors
  (for _index (range 0 (Math|Random|RandomIntegerinRange 5 12))
    ;[1 1 1] Find available node and get random node
    (bind _avail_nodes (CallFunction|GetAvailableNodes))
    (Utilities|Array|AddUnique (LocalVariables|GetIndex%20to%20Spawn) (Variables|/Game/CrossyRoad/Blueprints/BP_Base_Node.BP_Base_Node_C|Getindex (Utilities|Array|Get(acopy) _avail_nodes (Math|Random|RandomIntegerinRange 0 (Utilities|Array|LastIndex _avail_nodes))))))
  (for _array_element (LocalVariables|GetIndex%20to%20Spawn)
    (bind _returnvalue (Game|SpawnActorfromClass "/Game/CrossyRoad/Blueprints/Obstacles/BP_Lilypads.BP_Lilypads_C" (Math|Transform|MakeTransform (Math|Vector|MakeVector (.x (.Location (Math|Transform|BreakTransform (Transformation|GetActorTransform (Utilities|Array|Get(acopy) (Variables|Default|GetNodes) _array_element))))) (.y (.Location (Math|Transform|BreakTransform (Transformation|GetActorTransform (Utilities|Array|Get(acopy) (Variables|Default|GetNodes) _array_element))))) (- (.z (.Location (Math|Transform|BreakTransform (Transformation|GetActorTransform (Utilities|Array|Get(acopy) (Variables|Default|GetNodes) _array_element))))) (Variables|Default|GetLilypads%20Z%20Offset))) (.Rotation (Math|Transform|BreakTransform (Transformation|GetActorTransform (Utilities|Array|Get(acopy) (Variables|Default|GetNodes) _array_element)))) (.Scale (Math|Transform|BreakTransform (Transformation|GetActorTransform (Utilities|Array|Get(acopy) (Variables|Default|GetNodes) _array_element))))) "Undefined" 0 0))
    (Utilities|Array|Add (Variables|Default|GetObstacles) _returnvalue)
    (CallFunction|SetOccupiedNode true _array_element)))

(fn DestroyObstacles
  (for _array_element (Variables|Default|GetObstacles)
    (Actor|DestroyActor _array_element)))